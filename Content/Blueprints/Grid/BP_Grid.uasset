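; BP_Grid builds a tile grid centered on a point, storing tile data by index and forwarding it to a BP_GridVisual child actor for display.
; The construction script runs SpawnGrid, which sphere-traces each tile to snap its height and take its type from BP_GridModifier actors.
; Helpers test walkability and convert world locations to indices.
; Tick draws a debug sphere at the snapped cursor location, found by trace or grid-plane intersection.
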(event EventBeginPlay)

(event EventTick
  (params (DeltaSeconds :type Float%20%28single-precision%29))
  (bind _location (CallFunction|GetCursorLocation))
  (Rendering|Debug|DrawDebugSphere (Class|KismetMathLibrary|VectorSnappedtoGrid _location (.x (Variables|Default|GetGridTileSize))) 15.0 5 "(R=1.000000,G=0.991363,B=0.000000,A=1.000000)" 0.1 5.0))

(fn ConstructionScript
  (bind _asbp_grid_visual (Utilities|Casting|CastToBP_GridVisual (Variables|/Script/Engine.ChildActorComponent|GetChildActor (Variables|Default|GetCA_GridVisual))))
  (Variables|Default|SetGridVisual _asbp_grid_visual)
  (CallFunction|SpawnGrid (Variables|Default|GetGridCenterPos) (Variables|Default|GetGridTileSize) (Variables|Default|GetGridTileCount) true))

(fn SpawnGrid
  (params (CenterPos :type Vector) (TileSize :type Vector) (TileCount :type Vector%202D%20Structure) (UseEnvironment :type Boolean))
  ;[0.15 0.15 0.15 0.5] Establish Grid Pos and Visual
  (Variables|Default|SetGridCenterPos CenterPos)
  (Variables|Default|SetGridTileSize TileSize)
  (Variables|Default|SetGridTileCount TileCount)
  (CallFunction|DestroyGrid)
  (Default|InitializeGV (Variables|Default|GetGridVisual) self)
  ;[0.15 0.15 0.15 0.5] Get Bottom Left Corner (Starting) Location
  (Variables|Default|SetGridBLCornerPos (- (Variables|Default|GetGridCenterPos) (Math|Conversions|ToVector(Vector2D) (* (/ (Variables|Default|GetGridTileCount) 2.0) (Math|Conversions|ToVector2D(Vector) (Variables|Default|GetGridTileSize))))))
  ;[0.15 0.15 0.15 0.5] Determine Each Tile's Transform Starting From the Bottom Left Corner Based on Tile Size and Count
  (bind _result (Math|Integer|DecrementInt (Math|Float|Round (.x (Variables|Default|GetGridTileCount))))
    (:%20%20
      (for _index (range 0 _result)
        (LocalVariables|SetXIndex _index)
        (bind _result_2 (Math|Integer|DecrementInt (Math|Float|Round (.y (Variables|Default|GetGridTileCount))))
          (:%20%20
            (for _index_2 (range 0 _result_2)
              (LocalVariables|SetYIndex _index_2)
              (LocalVariables|SetIndex (Utilities|Struct|MakeIntPoint (LocalVariables|GetXIndex) (LocalVariables|GetYIndex)))
              (bind _returnvalue (Utilities|GetDataTableRow "/Game/Blueprints/Grid/DT_GridData.DT_GridData" "Grid")
                (:then
                  (LocalVariables|SetTileTransform (Math|Transform|MakeTransform (+ (+ (Variables|Default|GetGridBLCornerPos) (* (Variables|Default|GetGridTileSize) (Math|Vector|MakeVector (Math|Conversions|ToFloat(Integer) (LocalVariables|GetXIndex)) (Math|Conversions|ToFloat(Integer) (LocalVariables|GetYIndex)) 0.0))) "0.000000,0.000000,2.000000") "0, 0, 0" (/ (Variables|Default|GetGridTileSize) (.Size (Utilities|Struct|BreakS_GridData _returnvalue)))))
                  (if UseEnvironment
                    ;[0.15 0.15 0.15 0.5] Scan Environment for Ground
                    (bind (_tiletype _outlocation) (CallFunction|TraceforGround (.location (LocalVariables|GetTileTransform))))
                    ;[0.15 0.15 0.15 0.5] Add The Mesh
                    (CallFunction|AddGridTile (Utilities|Struct|MakeS_TileData (LocalVariables|GetIndex) _tiletype (Math|Transform|MakeTransform _outlocation (.rotation (LocalVariables|GetTileTransform)) (.scale (LocalVariables|GetTileTransform)))))
                    (else
                      ;[0.15 0.15 0.15 0.5] Add The Mesh
                      (CallFunction|AddGridTile (Utilities|Struct|MakeS_TileData (LocalVariables|GetIndex) "NewEnumerator1" (LocalVariables|GetTileTransform))))))))))))))

(fn DestroyGrid
  ;[0.15 0.15 0.15 0.5] Delete Data and Grid Visual
  (Utilities|Map|Clear (Variables|Default|GetGridTiles))
  (Default|DestroyGV (Variables|Default|GetGridVisual)))

(fn GetCursorLocation
  (params (PlayerIndex :type Integer))
  (bind _returnvalue (Game|GetPlayerController PlayerIndex))
  (bind _gridcenterpos (Variables|Default|GetGridCenterPos))
  (bind (_hitresult _returnvalue_2) (Game|Player|GetHitResultUnderCursorbyChannel _returnvalue "TraceTypeQuery3" false))
  (bind (_worldlocation _worlddirection) (Game|Player|ConvertMouseLocationToWorldSpace _returnvalue))
  (bind _returnvalue_3 (Class|KismetMathLibrary|MakePlanefromPointandNormal _gridcenterpos "0.000000,0.000000,1.000000"))
  (bind _returnvalue_4 (* _worlddirection 999999.0))
  (bind _returnvalue_5 (+ _worldlocation _returnvalue_4))
  (bind (_t _intersection _returnvalue_6) (Class|KismetMathLibrary|LinePlaneIntersection _worldlocation _returnvalue_5 _returnvalue_3))
  (if _returnvalue_2
    (return (.Location (Collision|BreakHitResult _hitresult)))
    (elif _returnvalue_6
      (return _intersection)
      (else
        (return "-999.000000,-999.000000,-999.000000")))))

(fn TraceforGround
  (params (Location :type Vector))
  (LocalVariables|SetRadius (/ (.x (Variables|Default|GetGridTileSize)) 3.0))
  (bind _outhits (Collision|MultiSphereTraceByChannel (+ Location "0.000000,0.000000,100.000000") (- Location "0.000000,0.000000,100.000000") (LocalVariables|GetRadius) "TraceTypeQuery4" false 0 "ForDuration"))
  (if (> (Utilities|Array|Length _outhits) 0)
    (LocalVariables|SetReturnType "NewEnumerator1")
    (for _array_element _outhits
      (bind _asbp_grid_modifier (Utilities|Casting|CastToBP_GridModifier (.HitActor (Collision|BreakHitResult _array_element))))
      (LocalVariables|SetReturnType (Variables|/Game/Blueprints/Grid/BP_GridModifier.BP_GridModifier_C|GetTileType _asbp_grid_modifier)))
    (return (LocalVariables|GetReturnType) (Math|Vector|MakeVector (.x Location) (.y Location) (Math|Float|SnapToGrid(Float) (- (.Z (Math|Vector|BreakVector (.Location (Collision|BreakHitResult _array_element)))) (LocalVariables|GetRadius)) (.z (Variables|Default|GetGridTileSize)))))
    (else
      (return "NewEnumerator0" Location))))

(fn IsTileWalkable
  (params (Type :type E_TileType%20Enum :default "NewEnumerator0"))
  (return (not (Utilities|Array|ContainsItem (Utilities|Array|MakeArray "NewEnumerator0" "NewEnumerator2") Type))))

(fn AddGridTile
  (params (Data :type S%20Tile%20Data%20Structure))
  (Utilities|Map|Add (Variables|Default|GetGridTiles) (.index Data) Data)
  (Default|UpdateTileVisual (Variables|Default|GetGridVisual) Data))

(fn GetTileIndexfromWorldLocation
  (params (Location :type Vector))
  (bind _output_get (LocalVariables|SetPosOnGrid (- Location (Variables|Default|GetGridBLCornerPos))))
  (LocalVariables|SetSnappedPosOnGrid (Math|Conversions|ToVector2D(Vector) (Class|KismetMathLibrary|VectorSnappedtoGrid _output_get (.x (Variables|Default|GetGridTileSize)))))
  (return (Class|KismetMathLibrary|ToIntPoint(Vector2D) (/ (LocalVariables|GetSnappedPosOnGrid) (Math|Conversions|ToVector2D(Vector) (Variables|Default|GetGridTileSize))))))