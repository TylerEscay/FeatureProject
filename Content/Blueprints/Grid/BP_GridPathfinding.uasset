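; BP_GridPathfinding is an actor Blueprint for grid pathfinding that so far only provides tile neighbor lookup, with no path search.
; GetNeighborIndexes offsets an IntPoint index to return the four orthogonally adjacent tiles, without diagonals.
; GetValidTileNeighbors passes that list through unchanged, with no bounds or walkability filtering.
; The event graph and construction script contain no logic.
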(event EventBeginPlay)

(event Collision|EventActorBeginOverlap
  (params (OtherActor :type Actor%20Object%20Reference)))

(event EventTick
  (params (DeltaSeconds :type Float%20%28single-precision%29)))

(fn ConstructionScript)

(fn GetValidTileNeighbors
  (params (Index :type Int%20Point%20Structure))
  (return (CallFunction|GetNeighborIndexes Index)))

(fn GetNeighborIndexes
  (params (Index :type Int%20Point%20Structure))
  (return (Utilities|Array|MakeArray (+ (Utilities|Struct|MakeIntPoint 1 0) Index) (+ (Utilities|Struct|MakeIntPoint 0 1) Index) (+ Index (Utilities|Struct|MakeIntPoint -1 0)) (+ Index (Utilities|Struct|MakeIntPoint 0 -1)))))