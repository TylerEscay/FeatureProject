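; BP_GridVisual is the actor that handles the visual representation of a grid.
; InitializeGV stores the grid reference and sets up its child-actor BP_GridMeshInstance with the flat mesh and border material from DT_GridData, using query-only collision.
; It then moves itself to the world origin and applies a Z ground offset.
; DestroyGV clears the mesh instances, while UpdateTileVisual is an empty stub.
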(event EventBeginPlay)

(event Collision|EventActorBeginOverlap
  (params (OtherActor :type Actor%20Object%20Reference)))

(event EventTick
  (params (DeltaSeconds :type Float%20%28single-precision%29)))

(fn ConstructionScript)

(fn InitializeGV
  (params (Grid :type BP%20Grid%20Object%20Reference))
  (Variables|Default|SetGrid Grid)
  (bind _asbp_grid_mesh_instance (Utilities|Casting|CastToBP_GridMeshInstance (Variables|/Script/Engine.ChildActorComponent|GetChildActor (Variables|Default|GetCA_GridMeshInstance))))
  (Variables|Default|SetGridMeshInstance _asbp_grid_mesh_instance)
  (bind _returnvalue (Utilities|GetDataTableRow "/Game/Blueprints/Grid/DT_GridData.DT_GridData" "Grid")
    (:then
      (Default|InitializeGMI :self (Variables|Default|GetGridMeshInstance) :NewMesh (.FlatMesh (Utilities|Struct|BreakS_GridData _returnvalue)) :Material (.BorderMaterial (Utilities|Struct|BreakS_GridData _returnvalue)) :Collision "QueryOnly")
      (Transformation|SetActorLocation "0, 0, 0" false false)
      (CallFunction|SetGroundOffset (Variables|Default|GetOffset)))))

(fn SetGroundOffset
  (params (Offset :type Float%20%28double-precision%29))
  (bind _returnvalue (Transformation|GetActorLocation))
  (bind _output_get (Variables|Default|SetOffset Offset))
  (Transformation|SetActorLocation (Math|Vector|MakeVector (.x _returnvalue) (.y _returnvalue) _output_get) false false))

(fn DestroyGV
  (Default|ClearInstances (Variables|Default|GetGridMeshInstance)))

(fn UpdateTileVisual)