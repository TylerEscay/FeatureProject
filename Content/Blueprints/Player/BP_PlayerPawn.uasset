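; BP_PlayerPawn is the player pawn, providing a zoomable spring arm view.
; On BeginPlay it caches player 0's BP_PlayerController and adds the IMC_PlayerControls Enhanced Input mapping context, stopping if the cast fails.
; IA_Zoom input, scaled by ZoomSpeed, adjusts the spring arm's target length within a clamped range.
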(event Input|EnhancedActionEvents|EnhancedInputActionIA_Zoom
  (params (ActionValue :type Float%20%28double-precision%29) (ElapsedSeconds :type Float%20%28double-precision%29) (TriggeredSeconds :type Float%20%28double-precision%29) (InputAction :type Input%20Action%20Object%20Reference :default "/Game/Inputs/Actions/IA_Zoom.IA_Zoom"))
  (bind _springarm (Variables|Default|GetSpringArm))
  (Variables|/Script/Engine.SpringArmComponent|SetTargetArmLength _springarm (Math|Float|Clamp(Float) (+ (* ActionValue (Variables|Default|GetZoomSpeed)) (Variables|/Script/Engine.SpringArmComponent|GetTargetArmLength _springarm)) 2.5e+02 3e+03)))

(event EventBeginPlay
  (bind _asbp_player_controller (Utilities|Casting|CastToBP_PlayerController (Game|GetPlayerController 0)))
  (bind _output_get (Variables|Default|SetPlayerController _asbp_player_controller))
  (Input|AddMappingContext (PlayerController|LocalPlayerSubsystems|GetEnhancedInputLocalPlayerSubsystem _output_get) "/Game/Inputs/IMC_PlayerControls.IMC_PlayerControls" 0 "(bIgnoreAllPressedKeysUntilRelease=True,bForceImmediately=False,bNotifyUserSettings=False)"))

(fn ConstructionScript)