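; Player actions Blueprint that handles mouse hover and click interaction with the tiles of BP_Grid.
; On BeginPlay it finds the grid and enables input for player 0.
; Each tick it moves a hover state to the tile under the cursor when that tile changes.
; Left and right clicks add and remove a second state on the hovered tile through raw mouse events; Enhanced Input setup exists but is disconnected.
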(event EventBeginPlay
  (bind _returnvalue (Actor|GetActorOfClass "/Game/Blueprints/Grid/BP_Grid.BP_Grid_C"))
  (Variables|Default|SetGrid _returnvalue)
  (Input|EnableInput (Game|GetPlayerController 0)))

(event EventTick
  (params (DeltaSeconds :type Float%20%28single-precision%29))
  (CallFunction|UpdateTileUnderCursor))

(event Input|MouseEvents|LeftMouseButton
  (params (Key :type Key%20Structure :default "None"))
  (:Pressed
    (Default|AddStatetoTile (Variables|Default|GetGrid) (Variables|Default|GetHoveredTile) "NewEnumerator2")))

(event Input|MouseEvents|RightMouseButton
  (params (Key :type Key%20Structure :default "None"))
  (:Pressed
    (Default|RemoveStatefromTile (Variables|Default|GetGrid) (Variables|Default|GetHoveredTile) "NewEnumerator2")))

(fn ConstructionScript)

(fn UpdateTileUnderCursor
  (bind _index (Default|GetTileIndexUnderCursor (Variables|Default|GetGrid)))
  (if (!= _index (Variables|Default|GetHoveredTile))
    (Default|RemoveStatefromTile (Variables|Default|GetGrid) (Variables|Default|GetHoveredTile) "NewEnumerator1")
    (bind _output_get (Variables|Default|SetHoveredTile _index))
    (Default|AddStatetoTile (Variables|Default|GetGrid) _output_get "NewEnumerator1")))